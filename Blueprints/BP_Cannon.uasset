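; BP_Cannon is an automatic cannon that fires projectiles repeatedly from BeginPlay.
; After a delay, it plays the shot sound, spawns a scaled BP_Projectile at its spawn point and starts the CannonFireAnim timeline.
; The timeline slides the cannon along its relative Y axis, and its event track loops back to the delay for the next shot.
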(event `self.ReceiveBeginPlay`
  (`KismetSystemLibrary.Delay` (`self.Time`) :!label _label)
  ; to make sound quieter when we're further from it
  (`AudioComponent.Play` (`self.CannonShot`) 0.0)
  (`self.SpwanProjectile`)
  (bind (_direction _cannonanim) (`Timeline|CannonFireAnim` :!via `PlayFromStart`)
    (:`Update`
      (`self.MoveCannon` _cannonanim))
    (:`CannonFireStart`
      (goto _label))))

(fn `MoveCannon`
  (params (CannonLocation :type "Float (double-precision)"))
  (`SceneComponent.K2_SetRelativeLocation` (`self.Cannon`) (`KismetMathLibrary.MakeVector` 0.0 CannonLocation) false false))

(fn `SpwanProjectile`
  (bind _spwanpoint (`self.SpwanPoint`))
  (`|SpawnActorFromClass` "/Game/Blueprints/BP_Projectile.BP_Projectile_C" (`KismetMathLibrary.MakeTransform` (`SceneComponent.K2_GetComponentLocation` _spwanpoint) (`SceneComponent.K2_GetComponentRotation` _spwanpoint) (`KismetMathLibrary.Conv_DoubleToVector` (`self.ProjectileScale`))) "Undefined" "MultiplyWithRoot" null null))

(fn `UserConstructionScript`)