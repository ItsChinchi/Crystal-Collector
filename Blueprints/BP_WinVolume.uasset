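; BP_WinVolume is an overlap volume that ends the level when the player enters it.
; If any BP_Crystal actors remain it quits the game; otherwise it opens the level following the current one in the LevelNames array.
; IsFinalLevel always returns false because its last-index comparison is unconnected, so the next-level lookup has no end-of-list guard.
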(event `self.ReceiveActorBeginOverlap`
  (params (OtherActor :type "Actor Object Reference"))
  (`/Game/Libraries/CC_MacroLibrary.Isplayer` OtherActor
    (:`IsPlayer`
      (if (`self.AreCrystalsRemaining`)
        (`KismetSystemLibrary.QuitGame` null "Quit")
        (else
          (`self.CompleteLevel`))))))

(fn `AreCrystalsRemaining`
  (returns (ReturnValue :type Boolean))
  (bind _outactors (`GameplayStatics.GetAllActorsOfClass` "/Game/Blueprints/BP_Crystal.BP_Crystal_C"))
  (return (> (`KismetArrayLibrary.Array_Length` _outactors) 0)))

(fn `CompleteLevel`
  (if (not (`self.IsFinalLevel`))
    (`self.LoadNextLevel`)))

(fn `GetCurrentLevelIndex`
  (returns (LevelIndex :type Integer))
  (bind _returnvalue (`GameplayStatics.GetCurrentLevelName` true))
  (return (`KismetArrayLibrary.Array_Find` (`self.LevelNames`) (`KismetStringLibrary.Conv_StringToName` _returnvalue))))

(fn `GetNextLevelName`
  (returns (Output :type Name))
  (return (`|GetArrayItem` (`self.LevelNames`) (+ (`self.GetCurrentLevelIndex`) 1))))

(fn `IsFinalLevel`
  (returns (ReturnValue :type Boolean))
  (return false))

(fn `LoadNextLevel`
  (`GameplayStatics.OpenLevel` (`self.GetNextLevelName`)))

(fn `UserConstructionScript`)