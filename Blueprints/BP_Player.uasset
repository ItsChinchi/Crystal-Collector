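; BP_Player is the player-controlled, physics-driven vehicle, steered like a tank with Enhanced Input forward/backward and turning actions.
; Input mixes into clamped left and right wheel forces, applied to the mesh at each wheel's location, while drive components fade in and out.
; A helper sets spring arm length and pitch.
; Any damage triggers a one-time camera fade, then reloads the current level.
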(event `self.ReceiveBeginPlay`
  ; to get the axis
  (`EnhancedInputSubsystemInterface.AddMappingContext` (pcsubsystem `EnhancedInputLocalPlayerSubsystem` (`GameplayStatics.GetPlayerController` 0)) "/Game/Inputs/Input_mapping.Input_mapping" 0 (struct)))

(event `EnhancedInput|/Game/Inputs/IA_Forward_Backward`
  (params (ActionValue :type "Float (double-precision)") (ElapsedSeconds :type "Float (double-precision)") (TriggeredSeconds :type "Float (double-precision)") (InputAction :type "InputAction Object Reference" :default "/Game/Inputs/IA_Forward_Backward.IA_Forward_Backward"))
  (bind _forwarddrive (`self.ForwardDrive`))
  (:`Triggered`
    (`self.SetWheelForce` ActionValue ActionValue (stale `EnhancedInput|/Game/Inputs/IA_Turning` ActionValue) (stale `EnhancedInput|/Game/Inputs/IA_Turning` ActionValue) :!label _label))
  (:`Started`
    (`AudioComponent.FadeIn` _forwarddrive 0.4 1.0 0.0 "Linear"))
  (:`Completed`
    (`AudioComponent.FadeOut` _forwarddrive 0.0 0.0 "Linear")
    (set `self.LeftWheelForce` 0.0 :!label _label_2)
    (set `self.RightWheelForce` 0.0)))

(event `EnhancedInput|/Game/Inputs/IA_Turning`
  (params (ActionValue :type "Float (double-precision)") (ElapsedSeconds :type "Float (double-precision)") (TriggeredSeconds :type "Float (double-precision)") (InputAction :type "InputAction Object Reference" :default "/Game/Inputs/IA_Turning.IA_Turning"))
  (bind _turndrive (`self.TurnDrive`))
  (:`Triggered`
    (goto _label))
  (:`Started`
    (`AudioComponent.FadeIn` _turndrive 0.4 1.0 0.0 "Linear"))
  (:`Completed`
    (`AudioComponent.FadeOut` _turndrive 0.0 0.0 "Linear")
    (goto _label_2)))

(event `self.ReceiveAnyDamage`
  (params (Damage :type "Float (single-precision)") (DamageType :type "DamageType Object Reference") (InstigatedBy :type "Controller Object Reference") (DamageCauser :type "Actor Object Reference"))
  (bind _fade_duration (`self.Fade_Duration`))
  ; destory the player and restart the game when hit
  (`/Engine/EditorBlueprintResources/StandardMacros.DoOnce` false
    (:`Completed`
      (`PlayerCameraManager.StartCameraFade` :`self` (`GameplayStatics.GetPlayerCameraManager` 0) :`ToAlpha` 1.0 :`Duration` _fade_duration)
      (`KismetSystemLibrary.Delay` _fade_duration)
      (bind _returnvalue (`GameplayStatics.GetCurrentLevelName` true))
      (`GameplayStatics.OpenLevel` (`KismetStringLibrary.Conv_StringToName` _returnvalue)))))

(fn `SetWheelForce`
  (params (A :type "Float (double-precision)") (A2 :type "Float (double-precision)") (B :type "Float (double-precision)") (B2 :type "Float (double-precision)"))
  (set `self.LeftWheelForce` (`KismetMathLibrary.FClamp` (+ A2 B2) -1.0))
  (set `self.RightWheelForce` (`KismetMathLibrary.FClamp` (- A B) -1.0))
  (`PrimitiveComponent.AddForceAtLocationLocal` (`self.PlayerMesh`) (`KismetMathLibrary.MakeVector` (* (`self.LeftWheelForce`) (`self.ForceMultiplier`))) (`SceneComponent.RelativeLocation` (`self.LEFTwheels`)) "None")
  (`PrimitiveComponent.AddForceAtLocationLocal` (`self.PlayerMesh`) (`KismetMathLibrary.MakeVector` (* (`self.RightWheelForce`) (`self.ForceMultiplier`))) (`SceneComponent.RelativeLocation` (`self.RIGHTwheels`)) "None"))

(fn `SpringArmm`
  (params (Distance :type "Float (double-precision)" :default 995.833008) (CameraPitch :type "Float (double-precision)" :default -39.0))
  (bind _springarm (`self.SpringArm`))
  (set `SpringArmComponent.TargetArmLength` Distance _springarm)
  (`SceneComponent.K2_SetWorldRotation` _springarm (`KismetMathLibrary.MakeRotator` 0.0 CameraPitch) false false))

(fn `UserConstructionScript`)