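; BP_Crystal is a collectible crystal actor that plays a pickup sound at its location and destroys itself when the player overlaps it.
; StoreStartingValues caches its start location, and MoveCrystalToPlayer lerps from that point to the first player pawn's current location by a supplied alpha.
; Neither function is called within this Blueprint, and the pickup adds no score or inventory here.
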(event `self.ReceiveActorBeginOverlap`
  (params (OtherActor :type "Actor Object Reference"))
  (`/Game/Libraries/CC_MacroLibrary.Isplayer` OtherActor
    (:`IsPlayer`
      (`GameplayStatics.PlaySoundAtLocation` "/Game/Sounds/GetCrystal.GetCrystal" (`self.K2_GetActorLocation`) (struct) 1.0 1.0 0.0 null null null null)
      (`self.K2_DestroyActor`))))

(fn `MoveCrystalToPlayer`
  (params (Alpha :type "Float (single-precision)"))
  (`self.K2_SetActorLocation` (`KismetMathLibrary.VLerp` (`self.CrystalStartLocation`) (`self.K2_GetActorLocation` (`GameplayStatics.GetPlayerPawn` 0)) Alpha)))

(fn `StoreStartingValues`
  (set `self.CrystalStartLocation` (`self.K2_GetActorLocation`)))

(fn `UserConstructionScript`)